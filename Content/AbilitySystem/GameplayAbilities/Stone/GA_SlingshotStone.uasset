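; GA_SlingshotStone is a gameplay ability that fires a stone from a slingshot toward the point under the mouse.
; On activation it takes the impact point from target data under the mouse and sends it to the avatar as a facing target.
; It plays the slingshot attack montage, then waits for the montage's stone gameplay event before spawning the projectile at that target.
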(event Ability|EventActivateAbility
  (bind _datahandle (|TargetDataUnderMouse)
    (:ValidDataHandle
      (Variables|Default|SetTargetLocation (.ImpactPoint (Collision|BreakHitResult (Ability|TargetData|GetHitResultfromTargetData _datahandle))))
      (Class|CombatInterface|UpdateFacingTarget(Message) (Ability|GetAvatarActorfromActorInfo) (Variables|Default|GetTargetLocation))
      (|PlayMontageandWaitProxy "None" "/Game/Assets/Enemies/Goblin/Animations/Slingshot/AM_Attack_Slingshot.AM_Attack_Slingshot" 1.0 "None" true 1.0 0.0 false
        (:then
          (Ability|Tasks|WaitGameplayEvent "(TagName=\"Event.Montage.Slingshot.Stone\")" 0
            (:EventReceived
              (Class|MPProjectileSpell|SpawnProjectile (Variables|Default|GetTargetLocation)))))))))

(event Ability|EventOnEndAbility
  (params (bWasCancelled :type Boolean)))